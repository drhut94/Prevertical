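; BlockTrap is a trap actor that, when used, spawns a batch of destructible blocks around its Box component.
; Use starts a looping timer that calls SpawnBlock, which counts NumBlocks down and clears the timer at zero.
; Each block spawns at a random offset from the box, with collision adjustment, and is appended to the Blocks array, which BeginPlay pre-sizes to NumBlocks.
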(event `self.ReceiveBeginPlay`
  (`parent.ReceiveBeginPlay`)
  (`KismetArrayLibrary.Array_Resize` (`self.Blocks`) (`self.NumBlocks`)))

(event `self.Use`
  (`KismetSystemLibrary.K2_SetTimer` null "SpawnBlock" 0.1 true))

(fn `SpawnBlock`
  (if (<= (`self.NumBlocks`) 0)
    (`KismetSystemLibrary.K2_ClearTimer` null "SpawnBlock")
    (else
      (`/Engine/EditorBlueprintResources/StandardMacros.DecrementInt` (`self.NumBlocks`)
        (:`  `
          (bind _returnvalue (`|SpawnActorFromClass` "/Game/FirstPersonBP/Blueprints/DestructibleObject.DestructibleObject_C" (`KismetMathLibrary.Conv_VectorToTransform` (+ (`SceneComponent.K2_GetComponentLocation` (`self.Box`)) (`KismetMathLibrary.MakeVector` (`KismetMathLibrary.RandomFloatInRange` -200.0 200.0) (`KismetMathLibrary.RandomFloatInRange` -200.0 200.0) (`KismetMathLibrary.RandomFloatInRange` -200.0 200.0)))) "AdjustIfPossibleButDontSpawnIfColliding" "OverrideRootScale" null null))
          (`KismetArrayLibrary.Array_Add` (`self.Blocks`) _returnvalue))))))

(fn `UserConstructionScript`
  (`parent.UserConstructionScript`))