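; DestructibleDoor is a door that, when grabbed, destroys itself along with the blocks of a BlockTrap in the level.
; On BeginPlay it disables normal destruction via CanBeDestroyed and DestructionVelocity, then caches the first BlockTrap found in the world.
; OnGrabb calls DestroyObject on itself, then sets each valid block to ignore the Destructible collision channel and destroys it.
; DestroyCubes is an empty stub.
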(event `self.ReceiveBeginPlay`
  (`parent.ReceiveBeginPlay`)
  (set `self.DestructionVelocity` -1.0)
  (set `self.CanBeDestroyed` false)
  (bind _outactors (`GameplayStatics.GetAllActorsOfClass` "/Game/Blueprints/Map/BlockTrap.BlockTrap_C"))
  (set `self.BlockTrap` (`|GetArrayItem` _outactors)))

(event `/Game/Interfaces/GrabbableObject.OnGrabb`
  (params (GrabPos :type "Vector Structure"))
  (bind _blocks (`/Game/Blueprints/Map/BlockTrap.Blocks` (`self.BlockTrap`)))
  (`self.DestroyObject`)
  (for (_array_element _array_index) _blocks
    (if (`KismetSystemLibrary.IsValid` _array_element)
      (bind _output (`|GetArrayItem` _blocks _array_index))
      (`PrimitiveComponent.SetCollisionResponseToChannel` (`DestructibleActor.DestructibleComponent` _output) "ECC_Destructible" "ECR_Ignore")
      (`self.DestroyObject` _output))))

(fn `DestroyCubes`)

(fn `UserConstructionScript`
  (`parent.UserConstructionScript`))